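; TrapPit_BP is an environment trap that picks a random damage type on BeginPlay: fire, electricity or a one-shot bomb.
; It hides its components, then shows the chosen type's plane, particle system or bomb mesh.
; On player overlap, fire and electricity repeat damage through a delay loop while the overlap lasts.
; The bomb instead spawns an enlarged emitter, applies damage once and destroys the actor.
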(event Collision|EventActorBeginOverlap
  (params (OtherActor :type Actor%20Object%20Reference))
  (bind _returnvalue (Game|GetPlayerCharacter 0))
  (bind _returnvalue_2 (Game|GetPlayerCharacter 0))
  (bind _continuousfiredamage (Variables|Default|GetContinuousFireDamage))
  (bind _damagetypeindex (Variables|Default|GetDamageTypeIndex))
  (bind _continuouselectricitydamage (Variables|Default|GetContinuousElectricityDamage))
  (bind _oneshotdamage (Variables|Default|GetOneShotDamage))
  (bind _returnvalue_3 (Collision|IsOverlappingActor _returnvalue_2 :!class /Script/Engine.Actor))
  (bind _returnvalue_4 (Utilities|Select :Index _damagetypeindex :Option%200 _continuousfiredamage :Option%201 _continuouselectricitydamage :Option%202 _oneshotdamage))
  ;[1 1 1] ApplyDamage
  (if (Variables|Default|GetAppliesContinuousDamage)
    (if _returnvalue_3 :!label _label
      (Utilities|IsValid (Game|GetPlayerCharacter 0)
        (:Is%20Valid
          (Game|Damage|ApplyDamage _returnvalue _returnvalue_4 0 0)
          (Utilities|FlowControl|Delay (Variables|Default|GetContinuousDamageRate))
          (goto _label))))
    (elif _returnvalue_3
      (Effects|SpawnEmitteratLocation (Utilities|Array|Get(acopy) (Variables|Default|GetDamageTypeParticleList) (Variables|Default|GetDamageTypeIndex)) (Transformation|GetWorldLocation (Variables|Default|GetParticleSystem)) "0, 0, 0" "3.000000,3.000000,3.000000")
      (Game|Damage|ApplyDamage _returnvalue _returnvalue_4 0 0)
      (Actor|DestroyActor))))

(event EventBeginPlay
  (Rendering|SetVisibility (Variables|Default|GetDefaultSceneRoot) false true)
  ;[1 1 1] RandomizeDamageType
  (bind _output_get (Variables|Default|SetDamageTypeIndex (Math|Random|RandomInteger (Utilities|Array|Length (Variables|Default|GetDamageTypeParticleList)))))
  (switch int _output_get
    (:Default
      ;[1 1 1] SetContinuousDamageParticles
      (Variables|Default|SetAppliesContinuousDamage true :!label _label)
      (Rendering|SetVisibility (Variables|Default|GetParticleSystem) true false)
      (Effects|Components|ParticleSystem|SetTemplate (Variables|Default|GetParticleSystem) (Utilities|Array|Get(acopy) (Variables|Default|GetDamageTypeParticleList) (Variables|Default|GetDamageTypeIndex))))
    (:0
      (Rendering|SetVisibility (Variables|Default|GetPlane) true false)
      (goto _label))
    (:1
      (goto _label))
    (:2
      ;[1 1 1] ShowBomb
      (Rendering|SetVisibility (Variables|Default|GetBomb) true false))))

(fn ConstructionScript)