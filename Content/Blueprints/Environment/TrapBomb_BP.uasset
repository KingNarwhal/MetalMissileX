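; TrapBomb_BP is an explosive environmental trap that detonates when the player character overlaps it or when it takes damage.
; On BeginPlay it randomly shows either a gas tank or a mine mesh as its appearance.
; Both triggers share one path that spawns an enlarged explosion at the Mine's location, calls ApplyDamage with no damaged actor specified, then destroys the trap.
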(event Game|Damage|EventAnyDamage
  (params (Damage :type Float%20%28single-precision%29) (DamageType :type Damage%20Type%20Object%20Reference) (InstigatedBy :type Controller%20Object%20Reference) (DamageCauser :type Actor%20Object%20Reference))
  ;[1 1 1] ApplyDamage
  (Effects|SpawnEmitteratLocation "/Game/StarterContent/Particles/P_Explosion.P_Explosion" (Transformation|GetWorldLocation (Variables|Default|GetMine)) "0, 0, 0" "3.000000,3.000000,3.000000")
  (Game|Damage|ApplyDamage 0 3e+01 0 0)
  (Actor|DestroyActor))

(event Collision|EventActorBeginOverlap
  (params (OtherActor :type Actor%20Object%20Reference))
  ;[1 1 1] ApplyDamage
  (if (== OtherActor (Game|GetPlayerCharacter 0))
    (Effects|SpawnEmitteratLocation "/Game/StarterContent/Particles/P_Explosion.P_Explosion" (Transformation|GetWorldLocation (Variables|Default|GetMine)) "0, 0, 0" "3.000000,3.000000,3.000000")
    (Game|Damage|ApplyDamage 0 3e+01 0 0)
    (Actor|DestroyActor)))

(event EventBeginPlay
  (Rendering|SetVisibility (Variables|Default|GetGasTank) false true)
  (Rendering|SetVisibility (Utilities|Select :Index (Math|Random|RandomInteger 2) :Option%200 (Variables|Default|GetGasTank) :Option%201 (Variables|Default|GetMine)) true true))

(fn ConstructionScript)