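; Missile launcher weapon Blueprint that fires a salvo of missiles, then enters a cooldown.
; Fire passes through a gate that closes while a looping timer spaces the missile count evenly across the shooting duration.
; Each shot spawns a BP_Missile at the spawn point, aimed by socket rotation with yaw flipped, assigns damage and shakes the player's camera.
; After the last missile, the timer clears and the gate reopens once the cooldown ends.
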(event Custom|StartFiring
  (Utilities|FlowControl|Gate false :!label _label
    (:Exit
      (Utilities|FlowControl|Sequence
        (:then_0
          (goto _label Close))
        (:then_1
          (bind _returnvalue (Utilities|Time|SetTimerbyEvent (delegate Custom|ShootMissile) (/ (Variables|Default|GetShootingDuration) (Math|Conversions|ToFloat(Integer) (Variables|Default|GetMissiles))) true)))))))

(event Custom|ShootMissile
  (bind _socket (Variables|Default|GetSocket))
  (bind _returnvalue (Transformation|GetSocketTransform _socket "None" "RTS_World"))
  (Math|Integer|IncrementInt (Variables|Default|GetShootCount)
    (:%20%20
      (bind _returnvalue_2 (Game|SpawnActorfromClass "/Game/Blueprints/Weapons/BP_Missile.BP_Missile_C" (Math|Transform|MakeTransform (Transformation|GetWorldLocation (Variables|Default|GetMissileSpawn)) (Math|Rotator|MakeRotator (.roll (.rotation _returnvalue)) (.pitch (.rotation _returnvalue)) (+ (.yaw (.rotation _returnvalue)) 1.8e+02)) "1,1,1") "Undefined" 0 0))
      (Variables|/Game/Blueprints/Weapons/BP_Missile.BP_Missile_C|SetDamage _returnvalue_2 (Variables|Default|GetMissileDamage))
      (bind _asthird_person_character (Utilities|Casting|CastToThirdPersonCharacter (Game|GetPlayerCharacter 0)))
      (Camera|PlayWorldCameraShake "/Game/Blueprints/UI/FireWeaponShake.FireWeaponShake_C" (Transformation|GetWorldLocation (Variables|/Game/Blueprints/Robot/ThirdPersonCharacter.ThirdPersonCharacter_C|GetFollowCamera _asthird_person_character)) 0.0 5e+02)
      (if (>= (Variables|Default|GetShootCount) (Variables|Default|GetMissiles))
        (Utilities|Time|ClearandInvalidateTimerbyHandle (stale Custom|StartFiring _returnvalue))
        (Variables|Default|SetShootCount 0)
        (Utilities|FlowControl|Delay (Variables|Default|GetCooldown))
        (Utilities|FlowControl|Gate false) ; enters at Open
      ))))

(event EventBeginPlay
  (|CallParentFunction) ; This node is disabled and will not be called.\nDrag off pins to build functionality.
)

(event Collision|EventActorBeginOverlap
  (params (OtherActor :type Actor%20Object%20Reference))
  (|CallParentFunction OtherActor) ; This node is disabled and will not be called.\nDrag off pins to build functionality.
)

(event EventTick
  (params (DeltaSeconds :type Float%20%28single-precision%29))
  (|CallParentFunction DeltaSeconds) ; This node is disabled and will not be called.\nDrag off pins to build functionality.
)

(fn ConstructionScript
  (|CallParentFunction))

(fn Fire
  (|CallParentFunction)
  (CallFunction|StartFiring))