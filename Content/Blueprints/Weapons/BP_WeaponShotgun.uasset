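; Shotgun weapon Blueprint, a child class that overrides Fire to launch pellets.
; Fire runs the parent logic, then spawns a BP_ShotgunPellets actor at the Socket component's world transform, with yaw flipped 180 degrees.
; The event graph holds only disabled default events, and the construction script just calls its parent.
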(event EventBeginPlay
  (|CallParentFunction) ; This node is disabled and will not be called.\nDrag off pins to build functionality.
)

(event Collision|EventActorBeginOverlap
  (params (OtherActor :type Actor%20Object%20Reference))
  (|CallParentFunction OtherActor) ; This node is disabled and will not be called.\nDrag off pins to build functionality.
)

(event EventTick
  (params (DeltaSeconds :type Float%20%28single-precision%29))
  (|CallParentFunction DeltaSeconds) ; This node is disabled and will not be called.\nDrag off pins to build functionality.
)

(fn ConstructionScript
  (|CallParentFunction))

(fn Fire
  (bind _socket (Variables|Default|GetSocket))
  (bind _returnvalue (Transformation|GetSocketTransform _socket "None" "RTS_World"))
  (|CallParentFunction)
  (Game|SpawnActorfromClass "/Game/Blueprints/Weapons/BP_ShotgunPellets.BP_ShotgunPellets_C" (Math|Transform|MakeTransform (.location _returnvalue) (Math|Rotator|MakeRotator (.roll (.rotation _returnvalue)) (.pitch (.rotation _returnvalue)) (+ (.yaw (.rotation _returnvalue)) 1.8e+02)) "1,1,1") "Undefined" 0 0))