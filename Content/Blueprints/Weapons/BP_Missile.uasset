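; BP_Missile is a homing projectile that damages what it hits.
; On BeginPlay it targets the mesh of the EnemyBase actor returned by GetActorOfClass, and a timeline ramps homing acceleration up from zero.
; The trail effect activates after a short delay.
; Capsule overlaps ignore other missiles and the player character; any other actor gets an explosion at its location and takes damage, then the missile destroys itself.
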(event OnComponentBeginOverlap(Capsule)
  (params (OverlappedComponent :type Primitive%20Component%20Object%20Reference) (OtherActor :type Actor%20Object%20Reference) (OtherComp :type Primitive%20Component%20Object%20Reference) (OtherBodyIndex :type Integer) (bFromSweep :type Boolean) (SweepResult :type Hit%20Result%20Structure%20%28by%20ref%29))
  (Utilities|IsValid OtherActor
    (:Is%20Valid
      (Utilities|Casting|CastToBP_Missile OtherActor
        (:CastFailed
          (if (not (== OtherActor (Game|GetPlayerCharacter 0)))
            (Effects|SpawnEmitteratLocation "/Game/StarterContent/Particles/P_Explosion.P_Explosion" (Transformation|GetActorLocation OtherActor))
            (Game|Damage|ApplyDamage OtherActor (Variables|Default|GetDamage) 0 0)
            (Actor|DestroyActor)))))))

(event EventBeginPlay
  (Utilities|FlowControl|Sequence
    (:then_0
      (bind _returnvalue (Actor|GetActorOfClass "/Game/Blueprints/Enemy/EnemyBase.EnemyBase_C"))
      (Utilities|IsValid _returnvalue
        (:Is%20Valid
          (Variables|/Script/Engine.ProjectileMovementComponent|SetHomingTargetComponent (Variables|Default|GetProjectileMovement) (Variables|/Script/Engine.Character|GetMesh _returnvalue))
          (bind _acceleration (Timeline|Acceleration PlayFromStart)
            (:Update
              (Variables|/Script/Engine.ProjectileMovementComponent|SetHomingAccelerationMagnitude (Variables|Default|GetProjectileMovement) (Math|Float|Lerp 0.0 5e+03 _acceleration)))))))
    (:then_1
      (Utilities|FlowControl|Delay 0.1)
      (Components|Activation|Activate (Variables|Default|GetTrail) false))))

(event Collision|EventActorBeginOverlap
  (params (OtherActor :type Actor%20Object%20Reference)))

(event EventTick
  (params (DeltaSeconds :type Float%20%28single-precision%29)))

(fn ConstructionScript)