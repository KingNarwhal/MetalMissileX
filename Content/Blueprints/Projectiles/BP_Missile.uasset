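; BP_Missile is a homing projectile that seeks the Scene component of a BP_Dummy actor found at BeginPlay.
; An Acceleration timeline ramps the ProjectileMovement homing acceleration from zero toward a fixed maximum, printing the value on each update.
; The capsule overlap event is empty and the ApplyDamage call is disconnected, so the Blueprint's graph deals no damage.
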(event OnComponentBeginOverlap(Capsule)
  (params (OverlappedComponent :type Primitive%20Component%20Object%20Reference) (OtherActor :type Actor%20Object%20Reference) (OtherComp :type Primitive%20Component%20Object%20Reference) (OtherBodyIndex :type Integer) (bFromSweep :type Boolean) (SweepResult :type Hit%20Result%20Structure%20%28by%20ref%29)))

(event EventBeginPlay
  (bind _returnvalue (Actor|GetActorOfClass "/Game/Blueprints/BP_Dummy.BP_Dummy_C"))
  (Variables|/Script/Engine.ProjectileMovementComponent|SetHomingTargetComponent (Variables|Default|GetProjectileMovement) (Variables|/Game/Blueprints/BP_Dummy.BP_Dummy_C|GetScene _returnvalue))
  (bind _acceleration (Timeline|Acceleration PlayFromStart)
    (:Update
      (bind _output_get (Variables|/Script/Engine.ProjectileMovementComponent|SetHomingAccelerationMagnitude (Variables|Default|GetProjectileMovement) (Math|Float|Lerp 0.0 5e+03 _acceleration)))
      (Development|PrintString (Utilities|String|ToString(Float) _output_get)))))

(event Collision|EventActorBeginOverlap
  (params (OtherActor :type Actor%20Object%20Reference)))

(event EventTick
  (params (DeltaSeconds :type Float%20%28single-precision%29)))

(fn ConstructionScript)