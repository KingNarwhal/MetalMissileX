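; Game mode for a fight game that runs the start menu and a timed round.
; On BeginPlay it freezes time with zero global time dilation, shows the start menu with the cursor, and binds its start event.
; Starting restores time, removes the menu and adds the HUD.
; Tick adds delta time to the elapsed time stored in FightGameStateBase and pauses the game once the round time limit is reached.
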(event Custom|event_start_fight
  (CallFunction|HideStartMenuandUnpauseGame)
  ;[1 1 1] add fight ui
  (bind _returnvalue (UserInterface|CreateWidget "/Game/Blueprints/UI/HUD_BP.HUD_BP_C"))
  (bind _output_get (Variables|Default|SetHUD _returnvalue))
  (UserInterface|Viewport|AddtoViewport _output_get 0))

(event EventBeginPlay
  (CallFunction|ShowStartMenuandPauseGame)
  ;[1 1 1] bind start event
  (EventDispatchers|BindEventtoOnStartFight (Variables|Default|GetStart_Menu) (delegate Custom|event_start_fight)))

(event EventTick
  (params (DeltaSeconds :type Float%20%28single-precision%29))
  (CallFunction|IncreaseTimeSinceStart DeltaSeconds)
  (if (>= (CallFunction|GetTimeSinceStart) (CallFunction|GetRoundTimeLimit))
    ;[1 1 1] endround
    (Game|SetGamePaused true)))

(fn ConstructionScript)

(fn GetTimeSinceStart
  (bind _asfight_game_state_base (Utilities|Casting|CastToFightGameStateBase (Game|GetGameState)))
  (return (Variables|/Game/Blueprints/GameState/FightGameStateBase.FightGameStateBase_C|Gettime_since_start _asfight_game_state_base)))

(fn GetRoundTimeLimit
  (bind _asfight_game_state_base (Utilities|Casting|CastToFightGameStateBase (Game|GetGameState)))
  (return (Variables|/Game/Blueprints/GameState/FightGameStateBase.FightGameStateBase_C|Getround_time_limit _asfight_game_state_base)))

(fn SetTimeSinceStart
  (params (time :type Float%20%28single-precision%29))
  (bind _asfight_game_state_base (Utilities|Casting|CastToFightGameStateBase (Game|GetGameState)))
  (Variables|/Game/Blueprints/GameState/FightGameStateBase.FightGameStateBase_C|Settime_since_start _asfight_game_state_base time))

(fn IncreaseTimeSinceStart
  (params (increase :type Float%20%28single-precision%29))
  (CallFunction|SetTimeSinceStart (+ increase (CallFunction|GetTimeSinceStart))))

(fn ShowStartMenuandPauseGame
  ;[1 1 1] show start menu and stop game
  (Utilities|Time|SetGlobalTimeDilation 0.0)
  (bind _returnvalue (UserInterface|CreateWidget "/Game/Blueprints/UI/Start_Menu_BP.Start_Menu_BP_C"))
  (bind _output_get (Variables|Default|SetStart_Menu _returnvalue))
  (UserInterface|Viewport|AddtoViewport _output_get 0)
  (Variables|/Script/Engine.PlayerController|SetbShowMouseCursor (Game|GetPlayerController 0) true))

(fn HideStartMenuandUnpauseGame
  (Utilities|Time|SetGlobalTimeDilation 1.0)
  (Widget|RemovefromParent (Variables|Default|GetStart_Menu)))