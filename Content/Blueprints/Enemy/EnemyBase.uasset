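; EnemyBase is an exploding enemy that detonates when the player touches it or its health runs out.
; Unless harmless, player overlap with DeathCapsule freezes its movement and plays a timeline that scales it up before detonation; death skips this wind-up.
; A DoOnce-guarded blast spawns effects, damages a still-overlapping player, shakes the camera and chain-detonates overlapping enemies before destroying itself.
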(event OnComponentBeginOverlap(DeathCapsule)
  (params (OverlappedComponent :type Primitive%20Component%20Object%20Reference) (OtherActor :type Actor%20Object%20Reference) (OtherComp :type Primitive%20Component%20Object%20Reference) (OtherBodyIndex :type Integer) (bFromSweep :type Boolean) (SweepResult :type Hit%20Result%20Structure%20%28by%20ref%29))
  (bind _charactermovement (Variables|Character|GetCharacterMovement))
  (Variables|Default|SetOtherActorOverlap OtherActor)
  (if (not (Variables|Default|GetIsHarmless))
    (if (== (Variables|Default|GetOtherActorOverlap) (Game|GetPlayerCharacter 0))
      ;[1 1 1] FreezeEnemy
      (Variables|/Script/Engine.CharacterMovementComponent|SetMaxWalkSpeed _charactermovement 0.0)
      (Variables|/Script/Engine.CharacterMovementComponent|SetRotationRate _charactermovement "0, 0, 0")
      (bind _newtrack_0 (Timeline|Timeline_0 PlayFromStart)
        (:Update
          ;[1 1 1] Grow
          (Transformation|SetActorScale3D (Math|Vector|Lerp(Vector) (Variables|Default|GetInitialScale) "1.500000,1.500000,1.500000" _newtrack_0)))
        (:Finished
          (Utilities|FlowControl|DoOnce false
            (:Completed
              (Utilities|FlowControl|Sequence
                (:then_0
                  ;[1 1 1] ExplosionFX
                  (Effects|SpawnEmitteratLocation "/Game/StarterContent/Particles/P_Explosion.P_Explosion" (Transformation|GetWorldLocation (Variables|Collision|GetCapsuleComponent)) "0, 0, 0" "5.000000,5.000000,5.000000"))
                (:then_1
                  ;[1 1 1] DamagePlayer
                  (if (Collision|IsOverlappingActor (Variables|Default|GetDeathCapsule) (Game|GetPlayerCharacter 0) :!class /Script/Engine.PrimitiveComponent)
                    (Game|Damage|ApplyDamage (Game|GetPlayerCharacter 0) (Variables|Default|GetExplosionDamage) 0 0)))
                (:then_2
                  ;[1 1 1] ScreenShake
                  (bind _asthird_person_character (Utilities|Casting|CastToThirdPersonCharacter (Game|GetPlayerCharacter 0)))
                  (Camera|PlayWorldCameraShake "/Game/Blueprints/UI/DamageStrongHealthShake.DamageStrongHealthShake_C" (Transformation|GetWorldLocation (Variables|/Game/Blueprints/Robot/ThirdPersonCharacter.ThirdPersonCharacter_C|GetFollowCamera _asthird_person_character)) 0.0 5e+02))
                (:then_3
                  ;[1 1 1] ExplodeOtherEnemy
                  (for _array_element (Collision|GetOverlappingActors "EnemyBase_C" :!class /Script/Engine.Actor)
                    (bind _asenemy_base (Utilities|Casting|CastToEnemyBase _array_element))
                    (CallFunction|Explode _asenemy_base))
                  (Actor|DestroyActor))))))))))

(event Custom|Explode
  (Utilities|FlowControl|DoOnce false
    (:Completed
      (Utilities|FlowControl|Sequence
        (:then_0
          ;[1 1 1] ExplosionFX
          (Effects|SpawnEmitteratLocation "/Game/StarterContent/Particles/P_Explosion.P_Explosion" (Transformation|GetWorldLocation (Variables|Collision|GetCapsuleComponent)) "0, 0, 0" "5.000000,5.000000,5.000000"))
        (:then_1
          ;[1 1 1] DamagePlayer
          (if (Collision|IsOverlappingActor (Variables|Default|GetDeathCapsule) (Game|GetPlayerCharacter 0) :!class /Script/Engine.PrimitiveComponent)
            (Game|Damage|ApplyDamage (Game|GetPlayerCharacter 0) (Variables|Default|GetExplosionDamage) 0 0)))
        (:then_2
          ;[1 1 1] ScreenShake
          (bind _asthird_person_character (Utilities|Casting|CastToThirdPersonCharacter (Game|GetPlayerCharacter 0)))
          (Camera|PlayWorldCameraShake "/Game/Blueprints/UI/DamageStrongHealthShake.DamageStrongHealthShake_C" (Transformation|GetWorldLocation (Variables|/Game/Blueprints/Robot/ThirdPersonCharacter.ThirdPersonCharacter_C|GetFollowCamera _asthird_person_character)) 0.0 5e+02))
        (:then_3
          ;[1 1 1] ExplodeOtherEnemy
          (for _array_element (Collision|GetOverlappingActors "EnemyBase_C" :!class /Script/Engine.Actor)
            (bind _asenemy_base (Utilities|Casting|CastToEnemyBase _array_element))
            (CallFunction|Explode _asenemy_base))
          (Actor|DestroyActor))))))

(event EventBeginPlay
  (Variables|Default|SetInitialScale "1.000000,1.000000,1.000000"))

(event Game|Damage|EventAnyDamage
  (params (Damage :type Float%20%28single-precision%29) (DamageType :type Damage%20Type%20Object%20Reference) (InstigatedBy :type Controller%20Object%20Reference) (DamageCauser :type Actor%20Object%20Reference))
  (Variables|Default|SetHealth (- (Variables|Default|GetHealth) Damage))
  (if (<= (Variables|Default|GetHealth) 0.0)
    (CallFunction|Explode)))

(fn ConstructionScript)